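; BP_ValidationSphere is a Blueprint in the VR painting canvas folder that prints a debug confirmation when hit, labelled as the validation sphere being grabbed.
; The Hit event proceeds only if the other actor casts to PlayerController, not a pawn, then passes an always-true branch.
; A OneCall flag, set on BeginPlay and cleared after printing, limits the message to once; no further validation logic exists.
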(event EventBeginPlay
  (|CallParentFunction)
  (Variables|Default|SetOneCall true))

(event EventTick
  (params (DeltaSeconds :type Float%20%28single-precision%29))
  (|CallParentFunction DeltaSeconds))

(event Collision|EventHit
  (params (MyComp :type Primitive%20Component%20Object%20Reference) (Other :type Actor%20Object%20Reference) (OtherComp :type Primitive%20Component%20Object%20Reference) (bSelfMoved :type Boolean) (HitLocation :type Vector :default "0, 0, 0") (HitNormal :type Vector :default "0, 0, 0") (NormalImpulse :type Vector :default "0, 0, 0") (Hit :type Hit%20Result%20Structure%20%28by%20ref%29))
  (Utilities|Casting|CastToPlayerController Other)
  (if true
    (if (Variables|Default|GetOneCall)
      (Development|PrintString "ValidationSphereGrabbed" true true "(R=0.037485,G=1.000000,B=0.007352,A=1.000000)" 2e+01)
      (Variables|Default|SetOneCall false))))

(fn ConstructionScript)