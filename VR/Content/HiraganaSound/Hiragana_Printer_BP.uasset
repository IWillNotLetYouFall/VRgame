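; Hiragana printer Blueprint that opens the Exercice widget on screen at BeginPlay and can show random hiragana with sound.
; DisplayRandomHiragana picks a random Hiraganas entry and passes its name to both WorldSprite and AudioManager, setting the sprite and playing the sound.
; Nothing in this graph's live flow calls that event; a one-second repeat loop around it is left disconnected.
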(event Custom|DisplayRandomHiragana
  (bind _hiraganas (Variables|Default|Gethiraganas))
  (bind _output_get (Variables|Default|SetrandomName (.name (Utilities|Array|Get(acopy) _hiraganas (Math|Random|RandomInteger (Utilities|Array|Length _hiraganas))))))
  (Default|SetSprite (Variables|Default|GetworldSprite) _output_get)
  (Default|PlaySound (Variables|Default|GetaudioManager) _output_get))

(event EventBeginPlay
  (bind _returnvalue (UserInterface|CreateWidget "/Game/HiraganaSound/Menu/exercice.exercice_C"))
  (UserInterface|Viewport|AddtoViewport _returnvalue 0))

(fn ConstructionScript)