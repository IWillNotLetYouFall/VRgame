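; Exercise dispatcher for the HiraganaSound game that presents a sequence of elements one at a time, each as a sprite with sound.
; SetSequence stores the sequence and starts it immediately, showing the first element through WorldSprite and AudioManager.
; Each DisplayNextElement call advances the index and presents the next element, clearing the running flag after the last one.
; The file contains no timer or input, so advancing depends on external calls.
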(event Custom|SetSequence
  (params (sequence :type Array%20of%20Strings))
  (Variables|Default|Setsequence sequence)
  (CallFunction|StartSequence))

(event Custom|StartSequence
  (if (> (Utilities|Array|Length (Variables|Default|Getsequence)) 0)
    (bind _output_get (Variables|Default|SetcurrentSequenceId 0))
    (Default|SetSprite (Variables|Default|GetworldSprite) (Utilities|Array|Get(acopy) (Variables|Default|Getsequence) _output_get))
    (Default|PlaySound (Variables|Default|GetaudioManager) (Utilities|Array|Get(acopy) (Variables|Default|Getsequence) _output_get))
    (Variables|Default|SetcurrentSequenceId (+ (Variables|Default|GetcurrentSequenceId) 1))
    (Variables|Default|SetisSequenceRuning true)))

(event Custom|DisplayNextElement
  (if (Variables|Default|GetisSequenceRuning)
    (Default|SetSprite (Variables|Default|GetworldSprite) (Utilities|Array|Get(acopy) (Variables|Default|Getsequence) (Variables|Default|GetcurrentSequenceId)))
    (Default|PlaySound (Variables|Default|GetaudioManager) (Utilities|Array|Get(acopy) (Variables|Default|Getsequence) (Variables|Default|GetcurrentSequenceId)))
    (bind _output_get (Variables|Default|SetcurrentSequenceId (+ (Variables|Default|GetcurrentSequenceId) 1)))
    (if (>= _output_get (Utilities|Array|Length (Variables|Default|Getsequence)))
      (Variables|Default|SetisSequenceRuning false))))

(event EventBeginPlay)

(fn ConstructionScript)